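; JogadorFps is a first-person player Blueprint that handles basic movement, camera look and jumping.
; Forward and right axis inputs add movement along vectors taken from the full control rotation, pitch included, rather than yaw alone.
; Look axes feed controller pitch and yaw directly, and the Jump action calls Jump on press, with no release handler.
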(event `InputAxis|MoveForward`
  (params (AxisValue :type "Float (single-precision)"))
  ;[0.3558 0.7326 0.8625] Move Player
  (`self.AddMovementInput` (`KismetMathLibrary.GetForwardVector` (`self.GetControlRotation`)) AxisValue))

(event `InputAxis|MoveRight`
  (params (AxisValue :type "Float (single-precision)"))
  ;[0.3558 0.7326 0.8625] Move Player
  (`self.AddMovementInput` (`KismetMathLibrary.GetRightVector` (`self.GetControlRotation`)) AxisValue))

(event `InputAction|Jump`
  (params (Key :type "Key Structure"))
  ;[0.3558 0.7326 0.8625] Move Player
  (:`Pressed`
    (`self.Jump`)))

(event `InputAxis|LookUp`
  (params (AxisValue :type "Float (single-precision)"))
  ;[1 1 1] Move Camera
  (`self.AddControllerPitchInput` AxisValue))

(event `InputAxis|LookRight`
  (params (AxisValue :type "Float (single-precision)"))
  ;[1 1 1] Move Camera
  (`self.AddControllerYawInput` AxisValue))

(fn `UserConstructionScript`)